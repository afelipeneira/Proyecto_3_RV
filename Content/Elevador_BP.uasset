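; Elevator Blueprint (Elevador) that animates a door and switches an indicator light; no cabin movement is implemented.
; Entering the B_Puerta trigger enables player input and plays a timeline that scales and offsets the door from its initial position.
; Leaving disables input and, if AbrirPuerta was set, plays a second door timeline.
; Pressing Y or entering the Luz trigger turns the light green; leaving Luz turns it red.
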(event OnComponentBeginOverlap(B_Puerta)
  (params (OverlappedComponent :type Primitive%20Component%20Object%20Reference) (OtherActor :type Actor%20Object%20Reference) (OtherComp :type Primitive%20Component%20Object%20Reference) (OtherBodyIndex :type Integer) (bFromSweep :type Boolean) (SweepResult :type Hit%20Result%20Structure%20%28by%20ref%29))
  (bind _puerta (Variables|Default|GetPuerta))
  (bind _relativescale3d (Variables|/Script/Engine.SceneComponent|GetRelativeScale3D _puerta))
  (Input|EnableInput (Game|GetPlayerController 0))
  (bind (_direction _multiplicador _newtrack_7) (Timeline|Sube%20puert Play)
    (:Update
      (Transformation|SetRelativeScale3D _puerta (Math|Vector|MakeVector (.x _relativescale3d) (.y _relativescale3d) _multiplicador))
      (Transformation|SetRelativeLocation _puerta (+ _newtrack_7 (Variables|Default|GetposicionIniPuerta)) false false)
      (Utilities|FlowControl|Delay 1.5))
    (:Finished
      _))
  (Variables|Default|Setabrir_Puerta true)
  (if (Variables|Default|Getsube_luz)
    _))

(event OnComponentEndOverlap(B_Puerta)
  (params (OverlappedComponent :type Primitive%20Component%20Object%20Reference) (OtherActor :type Actor%20Object%20Reference) (OtherComp :type Primitive%20Component%20Object%20Reference) (OtherBodyIndex :type Integer))
  (bind _puerta (Variables|Default|GetPuerta))
  (bind _puerta_2 (Variables|Default|GetPuerta))
  (bind _relativescale3d (Variables|/Script/Engine.SceneComponent|GetRelativeScale3D _puerta_2))
  (Input|DisableInput (Game|GetPlayerController 0))
  (if (Variables|Default|Getabrir_Puerta)
    (bind (_direction _multiplicador_2 _abre_2) (Timeline|Timeline_0 Play)
      (:Update
        (Transformation|SetRelativeScale3D _puerta (Math|Vector|MakeVector (.x _relativescale3d) (.y _relativescale3d) _multiplicador_2))
        (Transformation|SetRelativeLocation _puerta (+ (Variables|Default|GetposicionIniPuerta) _abre_2) false false)
        (Variables|Default|Setabrir_Puerta false)))))

(event OnComponentBeginOverlap(luz)
  (params (OverlappedComponent :type Primitive%20Component%20Object%20Reference) (OtherActor :type Actor%20Object%20Reference) (OtherComp :type Primitive%20Component%20Object%20Reference) (OtherBodyIndex :type Integer) (bFromSweep :type Boolean) (SweepResult :type Hit%20Result%20Structure%20%28by%20ref%29))
  (Rendering|Components|Light|SetLightColor (Variables|Default|GetPointLight) "(R=0.105615,G=1.000000,B=0.000000,A=1.000000)" true))

(event OnComponentEndOverlap(luz)
  (params (OverlappedComponent :type Primitive%20Component%20Object%20Reference) (OtherActor :type Actor%20Object%20Reference) (OtherComp :type Primitive%20Component%20Object%20Reference) (OtherBodyIndex :type Integer))
  (Rendering|Components|Light|SetLightColor (Variables|Default|GetPointLight) "(R=1.000000,G=0.000000,B=0.000000,A=1.000000)" true)
  (Variables|Default|Setsube_luz false))

(event Input|KeyboardEvents|U
  (params (Key :type Key%20Structure :default "AnyKey")))

(event Input|KeyboardEvents|Y
  (params (Key :type Key%20Structure :default "AnyKey"))
  (:Pressed
    (Variables|Default|Setsube_luz true)
    (if (Variables|Default|Getsube_luz)
      (Rendering|Components|Light|SetLightColor (Variables|Default|GetPointLight) "(R=0.105615,G=1.000000,B=0.000000,A=1.000000)" true))))

(fn ConstructionScript)